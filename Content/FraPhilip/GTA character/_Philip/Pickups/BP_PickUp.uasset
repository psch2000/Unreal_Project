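; BP_PickUp is a weapon pickup actor that offers itself to players who overlap its sphere.
; On the server, an overlap with a "Player"-tagged actor waits briefly, then passes the pickup through SetPickupMessage; end overlap does nothing.
; Events disable sphere collision against multi-spawning and destroy the actor on pickup.
; Getters expose weapon type, blendspace and self-reference, alongside a ShootWeapon override and an empty ShootWeaponDab.
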(event `self.ShootWeapon`
  ;[1 1 1] Shoot Override
  (`self.ShootWeapon`))

(event `ShootWeaponDab`
  ;[1 1 1] Shoot Override
)

(event `DisableCollision`
  ;[1 1 1] Disables collision //To prevent multi spawning
  (`PrimitiveComponent.SetCollisionEnabled` (`self.Sphere`) "NoCollision"))

(event `RemovePickupFromWorld`
  ;[1 1 1] Removes actor upon pickup
  (`self.K2_DestroyActor`))

(event `self.Sphere.OnComponentBeginOverlap`
  (params (OverlappedComponent :type "PrimitiveComponent Object Reference") (OtherActor :type "Actor Object Reference") (OtherComp :type "PrimitiveComponent Object Reference") (OtherBodyIndex :type Integer) (bFromSweep :type Boolean) (SweepResult :type "HitResult Structure (by ref)"))
  ;[1 1 1] Enables player to pickup when colliding
  (`/Engine/EditorBlueprintResources/ActorMacros.Switch Has Authority`
    (:`Authority`
      (if (`self.ActorHasTag` OtherActor "Player")
        (`KismetSystemLibrary.Delay` 0.2)
        (message `/Game/_Philip/Interfaces/INT_PlayerCharacter.SetPickup` OtherActor self)))))

(event `self.Sphere.OnComponentEndOverlap`
  (params (OverlappedComponent :type "PrimitiveComponent Object Reference") (OtherActor :type "Actor Object Reference") (OtherComp :type "PrimitiveComponent Object Reference") (OtherBodyIndex :type Integer))
  (`/Engine/EditorBlueprintResources/ActorMacros.Switch Has Authority`))

(fn `BlendSpaceInt`
  (returns (int :type Integer))
  (return (`self.Blendspace`)))

(fn `GetWeaponType`
  (returns (WeaponType :type "/Game/_Philip/E_WeaponType Enum"))
  (return (`self.WeaponType`)))

(fn `PIckupRef`
  (returns (PickupRef :type "/Game/FraPhilip/GTA character/_Philip/Pickups/BP_PickUp Object Reference"))
  (return self))

(fn `UserConstructionScript`)